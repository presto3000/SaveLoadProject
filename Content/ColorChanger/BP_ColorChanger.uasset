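; BP_ColorChanger is an actor whose static mesh switches to a random color whenever something begins overlapping it.
; On BeginPlay it creates a dynamic instance of M_ColorChanger and applies the stored LinearColor to its Color parameter.
; Each overlap stores a new random color in that variable and updates the material.
; GetUniqueSaveName returns a fixed name, and comments mark loading and saving points, though no save calls appear here.
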(event `self.ReceiveBeginPlay`
  (bind _returnvalue (`KismetMaterialLibrary.CreateDynamicMaterialInstance` "/Game/ColorChanger/M_ColorChanger.M_ColorChanger"))
  (bind _output_get (set `self.MaterialInstance` _returnvalue))
  (`PrimitiveComponent.SetMaterial` (`self.StaticMesh`) 0 _output_get)
  ;[1 1 1] Loading
  (`MaterialInstanceDynamic.SetVectorParameterValue` (`self.MaterialInstance`) "Color" (`self.Linear Color`)))

(event `self.StaticMesh.OnComponentBeginOverlap`
  (params (OverlappedComponent :type "PrimitiveComponent Object Reference") (OtherActor :type "Actor Object Reference") (OtherComp :type "PrimitiveComponent Object Reference") (OtherBodyIndex :type Integer) (bFromSweep :type Boolean) (SweepResult :type "HitResult Structure (by ref)"))
  ;[1 1 1] Saving
  (bind _output_get (set `self.Linear Color` (make `LinearColor` (`KismetMathLibrary.RandomFloatInRange` 0.0 1.0) (`KismetMathLibrary.RandomFloatInRange` 0.0 1.0) (`KismetMathLibrary.RandomFloatInRange` 0.0 1.0))))
  (`MaterialInstanceDynamic.SetVectorParameterValue` (`self.MaterialInstance`) "Color" _output_get))

(fn `GetUniqueSaveName`
  (returns (ReturnValue :type String))
  (return "ColorChanger"))

(fn `UserConstructionScript`)